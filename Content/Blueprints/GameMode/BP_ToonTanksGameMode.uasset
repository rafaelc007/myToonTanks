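; Game mode for Toon Tanks that handles the start and end screens of a match.
; StartGame creates the start-game widget and adds it to the viewport.
; GameOver creates the end-game widget, sets its text and color from the WonGame flag (blue for a win, red for a loss), then displays it.
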(event EventGameOver
  (params (bWonGame :type Boolean))
  (bind _returnvalue (UserInterface|CreateWidget "/Game/Blueprints/Widgets/WBP_EndGameWidget.WBP_EndGameWidget_C"))
  (Rendering|Components|TextRender|SetText (Variables|/Game/Blueprints/Widgets/WBP_EndGameWidget.WBP_EndGameWidget_C|GetDisplayText _returnvalue) (select bWonGame "Winner" "You lose"))
  (Appearance|SetColorandOpacity (Variables|/Game/Blueprints/Widgets/WBP_EndGameWidget.WBP_EndGameWidget_C|GetDisplayText _returnvalue) (select bWonGame (Utilities|Struct|MakeSlateColor "(R=0.000000,G=0.009012,B=1.000000,A=1.000000)") (Utilities|Struct|MakeSlateColor "(R=1.000000,G=0.028483,B=0.028483,A=1.000000)")) :!class /Script/UMG.TextBlock)
  (UserInterface|Viewport|AddtoViewport _returnvalue 0))

(event EventStartGame
  (bind _returnvalue (UserInterface|CreateWidget "/Game/Blueprints/Widgets/WBP_StartGamewidget.WBP_StartGamewidget_C"))
  (UserInterface|Viewport|AddtoViewport _returnvalue 0))

(fn ConstructionScript)